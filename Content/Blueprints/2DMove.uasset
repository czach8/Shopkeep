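; 2D customer actor that walks a waypoint loop through the shop and stops to barter for a displayed item.
; A self-restarting timeline lerps between waypoints, choosing directional flipbooks by position index.
; Each customer gets a random persona whose item list is matched against display slots, opening barter and dialogue at the stop, with Metal meaning no item.
; Completed loops decrement the customer count; closing spends energy through W_Main, and ReOpen adds customers.
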(event `FindNewCustomer`
  (bind _output_get (set `self.PersonSelected` (`KismetMathLibrary.RandomInteger` 5)))
  (switch `int` _output_get
    (:`0`
      (set `self.BehaviorCurrent` null))
    (:`1`
      (set `self.BehaviorCurrent` null))
    (:`2`
      (set `self.BehaviorCurrent` null))
    (:`3`
      (set `self.BehaviorCurrent` null))
    (:`4`
      (set `self.BehaviorCurrent` null)))
  (set `self.generosityVal` 0.0)
  (set `self.found` false)
  (for _array_element _ :!label _label
    (for _array_element_2 (`/Game/Blueprints/BP_Display.slots` (`self.Display`))
      (bind _itemclass (break `/Game/Blueprints/S_ItemSlot` _array_element_2))
      (if (== _itemclass _array_element)
        (set `self.found` true)
        (set `self.wantedItem` _itemclass)
        (goto _label :!via `Break`))))
  (if (not (`self.found`))
    (set `self.wantedItem` "/Game/Blueprints/Item_Classes/Metal.Metal_C")))

(event `CloseShop`
  (if (`self.shouldMinus`)
    (set `self.shouldMinus` false)
    (bind _foundwidgets (`WidgetBlueprintLibrary.GetAllWidgetsOfClass` "/Game/GUI/W_Main.W_Main_C"))
    (for _array_element _foundwidgets
      (`/Game/GUI/W_Main.MinusEnergy` _array_element)
      (if (> (`/Game/GUI/W_Energy.EnergyAmount` (`/Game/GUI/W_Main.W_Energy` _array_element)) 0)
        (`/Game/GUI/W_Main.EnableActions` _array_element)))))

(event `AnimationController`
  (bind _cont (`self.Cont`))
  (if (`self.Stop`)
    (if (`self.ShouldStop`)
      (`SceneComponent.SetVisibility` (`self.sprite`) false false)
      (`SceneComponent.SetVisibility` (`self.CustomerSprite`) true true)
      (else
        (`SceneComponent.SetVisibility` (`self.sprite`) true true :!label _label_2)
        (`SceneComponent.SetVisibility` (`self.CustomerSprite`) false false)
        (set `self.Cont` true)
        (for _array_element (`self.UpVectors`)
          (if (== _array_element (`self.position`))
            (`PaperFlipbookComponent.SetFlipbook` (`self.sprite`) "/Game/Assets/Sprites/HoodedAnimation/FB_Back.FB_Back")
            (set `self.Cont` false)))
        (if _cont
          (for _array_element_2 (`self.LeftVectors`)
            (if (== _array_element_2 (`self.position`))
              (`PaperFlipbookComponent.SetFlipbook` (`self.sprite`) "/Game/Assets/Sprites/HoodedAnimation/FB_Left.FB_Left")
              (set `self.Cont` false)))
          (if _cont
            (for _array_element_3 (`self.DownVectors`)
              (if (== _array_element_3 (`self.position`))
                (`PaperFlipbookComponent.SetFlipbook` (`self.sprite`) "/Game/Assets/Sprites/HoodedAnimation/FB_Forward.FB_Forward")
                (set `self.Cont` false)))
            (if _cont
              (for _array_element_4 (`self.RightVectors`)
                (if (== _array_element_4 (`self.position`))
                  (`PaperFlipbookComponent.SetFlipbook` (`self.sprite`) "/Game/Assets/Sprites/HoodedAnimation/FB_Right.FB_Right")
                  (set `self.Cont` false))))))))
    (else
      (goto _label_2))))

(event `ReOpen`
  (params (NewParam :type Integer))
  ;[1 1 1] Adds to the number of people
  (set `self.NumberOfPeople` (+ NewParam (`self.NumberOfPeople`)))
  (set `self.shouldMinus` true)
  (bind _foundwidgets (`WidgetBlueprintLibrary.GetAllWidgetsOfClass` "/Game/GUI/W_Main.W_Main_C"))
  (for _array_element _foundwidgets
    (`/Game/GUI/W_Main.DisableActions` _array_element)))

(event `NewCustomer2`
  ;[1 1 1] Checks if any of the items match
  (`self.getItems`)
  (set `self.found` false)
  (`self.getDisplay`)
  (`/Game/GUI/W_Barter.UpdateAttempts` (`self.Barter`))
  (for _array_element (`self.ItemArray`) :!label _label_3
    (for _array_element_2 (`/Game/Blueprints/BP_Display.slots` (`self.Display`))
      (bind _itemclass (break `/Game/Blueprints/S_ItemSlot` _array_element_2))
      (if (== _itemclass _array_element)
        (set `self.found` true)
        (set `self.wantedItem` _itemclass)
        (goto _label_3 :!via `Break`))))
  (if (not (`self.found`))
    (set `self.wantedItem` "/Game/Blueprints/Item_Classes/Metal.Metal_C")))

(event `GoodDay`
  (set `self.position` (+ (`self.position`) 1))
  (set `self.Stop` false)
  (`self.NewCustomer2`))

(event `gotItem`
  (set `self.WantedItem` "/Game/Blueprints/Item_Classes/Metal.Metal_C"))

(event `getDisplay`
  ;[1 1 1] Sets the barter and display
  (bind _foundwidgets (`WidgetBlueprintLibrary.GetAllWidgetsOfClass` "/Game/GUI/W_Main.W_Main_C"))
  (for _array_element _foundwidgets
    (set `self.Barter` (`/Game/GUI/W_Main.BarterMenu` _array_element))
    (set `self.Display` (`/Game/GUI/Display/W_Display.Display` (`/Game/GUI/W_Main.W_Display` _array_element)))
    (set `self.Dialogue` (`/Game/GUI/W_Main.W_Dialogue` _array_element))))

(event `GoToNextLocation`
  (bind _numberofpeople (`self.NumberOfPeople`))
  (bind _dialogue (`self.Dialogue`))
  (bind _sprite (`self.sprite`))
  (bind _barter (`self.Barter`))
  (bind _returnvalue (+ (`self.position`) 1))
  (bind (_direction _driver) (`Timeline|MoveTimeLine` :!via `PlayFromStart`)
    (:`Update`
      (`self.AnimationController`)
      (if (`self.start`)
        (set `self.start` false)
        (`self.NewCustomer2`))
      ;[1 1 1] Moving
      (if (> (`self.NumberOfPeople`) 0)
        (if (`self.Stop`)
          (set `self.ShouldStop` true)
          ;[1 1 1] Updates Barter and sets Visibility
          (if (== (`self.WantedItem`) "/Game/Blueprints/Item_Classes/Metal.Metal_C")
            (set `self.Stop` false)
            (set `self.ShouldStop` false)
            (else
              (`/Game/GUI/W_Barter.Update Barter Info` _barter (`self.WantedItem`) (`self.generosityVal`))
              (`Widget.SetVisibility` _barter "Visible")
              (if (`self.barterStart`)
                (`/Game/GUI/W_Dialogue.UpdateDialogueImage` _dialogue (`KismetArrayLibrary.Array_Get` (`self.picture`) (`self.PersonSelected`)))
                (`Widget.SetVisibility` _dialogue "HitTestInvisible")
                (`/Game/GUI/W_Dialogue.UpdateDialogue` _dialogue 0 (`self.WantedItem`))
                (set `self.barterStart` false))))
          (else
            (if (== (`self.position`) 0)
              (`SceneComponent.K2_SetRelativeLocation` _sprite (`KismetMathLibrary.VLerp` (0.0 0.0 0.0) (`KismetArrayLibrary.Array_Get` (`self.LocationVecs`) (`self.position`)) _driver) false false)
              (`SceneComponent.K2_SetRelativeLocation` (`self.CustomerSprite`) (`KismetMathLibrary.VLerp` (0.0 0.0 0.0) (`KismetArrayLibrary.Array_Get` (`self.LocationVecs`) (`self.position`)) _driver) false false)
              (else
                (`SceneComponent.K2_SetRelativeLocation` _sprite (`KismetMathLibrary.VLerp` (`KismetArrayLibrary.Array_Get` (`self.LocationVecs`) (- (`self.position`) 1)) (`KismetArrayLibrary.Array_Get` (`self.LocationVecs`) (`self.position`)) _driver) false false)
                (`SceneComponent.K2_SetRelativeLocation` (`self.CustomerSprite`) (`KismetMathLibrary.VLerp` (`KismetArrayLibrary.Array_Get` (`self.LocationVecs`) (- (`self.position`) 1)) (`KismetArrayLibrary.Array_Get` (`self.LocationVecs`) (`self.position`)) _driver) false false)))
            (if (== (`self.position`) (`self.stopPos`))
              (set `self.Stop` true)
              (else
                (set `self.Stop` false)))))))
    (:`Finished`
      ;[1 1 1] Selects Next Node and Checks if it shuld continue moving
      (if (== (`self.position`) 8)
        (`Widget.SetVisibility` (`self.Dialogue`) "Hidden")
        (if (> _numberofpeople 0)
          (set `self.NumberOfPeople` (- _numberofpeople 1))
          (else
            (`self.CloseShop`)))
        (`self.NewCustomer2`))
      (if (> (`self.NumberOfPeople`) 0)
        (if (`self.Stop`)
          (if (`self.ShouldStop`)
            (`self.GoToNextLocation` :!label _label_4)
            (else
              (if (> _returnvalue 8) :!label _label_5
                (set `self.position` 0)
                (else
                  (set `self.position` _returnvalue)))
              (`self.GoToNextLocation`)))
          (else
            (goto _label_5)))
        (else
          (goto _label_4))))))

(event `self.ReceiveTick`
  (params (DeltaSeconds :type "Float (single-precision)")))

(event `self.ReceiveBeginPlay`)

(fn `getItems`
  (bind _output_get (set `self.PersonSelected` (`KismetMathLibrary.RandomInteger` 5)))
  (bind (_newparam1 _newparam) (`/Game/Blueprints/Behaviors/BP_BehaviorMas.getCustomerItemArray` (`self.BehaviorCurrent`) _output_get))
  (set `self.ItemArray` _newparam1)
  (set `self.generosityVal` _newparam)
  (set `self.barterStart` true))

(fn `Move`
  (set `self.Stop` false))

(fn `UserConstructionScript`
  (`SceneComponent.K2_SetRelativeLocation` (`self.CustomerSprite`) (`KismetMathLibrary.SelectVector` (`KismetArrayLibrary.Array_Get` (`self.LocationVecs`) (`self.stopPos`)) (0.0 0.0 0.0) (`self.TestEndLoc`)) false false))