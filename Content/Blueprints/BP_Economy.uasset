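; BP_Economy is a Blueprint that tracks the player's money across in-game days.
; Add and Subtract adjust the Wallet, accumulate daily gain and loss totals, and refresh the wallet widget.
; EndDay deducts the tax rate as a flat amount and returns whether the balance has gone negative.
; NewDay clears the daily totals and SetTax changes the tax, with no event-driven logic.
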(fn `Add`
  (params (amount :type Integer))
  (locals (localAmount :type Integer))
  (bind _output_get (set `local.localAmount` amount))
  (set `self.dailyGain` (+ _output_get (`self.dailyGain`)))
  (set `self.wallet` (+ (`local.localAmount`) (`self.wallet`)))
  (`/Game/GUI/W_Wallet.UpdateWallet` (`self.walletWidget`)))

(fn `EndDay`
  (returns (under :type Boolean))
  (bind _output_get (set `self.wallet` (- (`self.wallet`) (`self.taxRate`))))
  (`/Game/GUI/W_Wallet.UpdateWallet` (`self.walletWidget`))
  (if (< _output_get 0)
    (return true)
    (else
      (return false))))

(fn `NewDay`
  (set `self.dailyLoss` 0)
  (set `self.dailyGain` 0))

(fn `SetTax`
  (params (newTax :type Integer))
  (set `self.taxRate` newTax))

(fn `Subtract`
  (params (loss :type Integer))
  (locals (localAmount :type Integer))
  (bind _output_get (set `local.localAmount` loss))
  (set `self.dailyLoss` (+ _output_get (`self.dailyLoss`)))
  (set `self.wallet` (- (`self.wallet`) (`local.localAmount`)))
  (`/Game/GUI/W_Wallet.UpdateWallet` (`self.walletWidget`)))

(fn `UserConstructionScript`)