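; BP_Inventory is a slot-based inventory that creates the main HUD widget on BeginPlay and registers it with Economy.
; Items are stored as class and amount pairs, with item data read from class defaults.
; AddItem recursively spreads amounts across free stacks and empty slots, returning true even if overflow fails to fit.
; Removal works by index or by class across slots, and changes refresh slot widgets and the crafting detail window.
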(event `self.ReceiveBeginPlay`
  (`KismetArrayLibrary.Array_Resize` (`self.slots`) (`self.amountOfSlots`))
  (bind _returnvalue (`|CreateWidget` "/Game/GUI/W_Main.W_Main_C" null self (`self.SlotsPerRow`) (`self.economy`)))
  (bind _output_get (set `self.MainWidget` _returnvalue))
  (set `self.Inventory Widget` (`/Game/GUI/W_Main.InventoryWidget` _output_get))
  (`UserWidget.AddToViewport` (`self.MainWidget`) 0)
  (set `/Game/Blueprints/BP_Economy.main` (`self.MainWidget`) (`self.economy`)))

(event `UpdateSlotAtIndex`
  (params (Index :type Integer))
  (`/Game/GUI/Inventory/W_Itemslot.updateSlot` (`KismetArrayLibrary.Array_Get` (`/Game/GUI/Inventory/W_Inventory.SlotsWidgets` (`self.Inventory Widget`)) Index)))

(fn `addItem`
  (params (itemClass :type "/Game/Blueprints/Item_Classes/BP_ItemMaster Class Reference") (amount :type Integer))
  (returns (success :type Boolean))
  (locals (localClass :type "/Game/Blueprints/Item_Classes/BP_ItemMaster Class Reference") (localAmount :type Integer) (foundIndex :type Integer))
  (bind (_item_itemclass _item_amount) (break `/Game/Blueprints/S_ItemSlot` (`KismetArrayLibrary.Array_Get` (`self.slots`) (`local.foundIndex`))))
  (bind _returnvalue (+ _item_amount (`local.localAmount`)))
  (set `local.localClass` itemClass)
  (set `local.localAmount` amount)
  (if (`.Stackable_27_55C25E0840B824F764E0AA9FCC62413B` (break `/Game/Blueprints/S_Item` (defaults `/Game/Blueprints/BP_Inventory` itemClass)))
    (bind (_found _index) (`self.findFreeStack` (`local.localClass`)))
    (if _found
      (set `local.foundIndex` _index)
      (if (> _returnvalue (`self.maxStackSize`))
        (set `local.localAmount` (- _returnvalue (`self.maxStackSize`)))
        (`KismetArrayLibrary.Array_Set` (`self.slots`) (`local.foundIndex`) (make `/Game/Blueprints/S_ItemSlot` (`local.localClass`) (`self.maxStackSize`)))
        (`self.addItem` (`local.localClass`) (`local.localAmount`))
        (`self.UpdateSlotAtIndex` (`local.foundIndex`))
        (`self.UpdateCraftingMenu`)
        (return true)
        (else
          (`KismetArrayLibrary.Array_Set` (`self.slots`) (`local.foundIndex`) (make `/Game/Blueprints/S_ItemSlot` (`local.localClass`) _returnvalue))
          (`self.UpdateSlotAtIndex` (`local.foundIndex`))
          (`self.UpdateCraftingMenu`)
          (return true)))
      (else
        (bind (_index_2 _found_2) (`self.getEmptySlot`))
        (if _found_2
          (bind _output_get (set `local.foundIndex` _index_2))
          (if (> (`local.localAmount`) (`self.maxStackSize`))
            (`KismetArrayLibrary.Array_Set` (`self.slots`) _output_get (make `/Game/Blueprints/S_ItemSlot` (`local.localClass`) (`self.maxStackSize`)))
            (`self.UpdateSlotAtIndex` (`local.foundIndex`))
            (`self.addItem` (`local.localClass`) (- (`local.localAmount`) (`self.maxStackSize`)))
            (`self.UpdateCraftingMenu`)
            (return true)
            (else
              (`KismetArrayLibrary.Array_Set` (`self.slots`) (`local.foundIndex`) (make `/Game/Blueprints/S_ItemSlot` (`local.localClass`) (`local.localAmount`)))
              (`self.UpdateSlotAtIndex` (`local.foundIndex`))
              (`self.UpdateCraftingMenu`)
              (return true)))
          (else
            (return false)))))
    (else
      (bind (_index_3 _found_3) (`self.getEmptySlot`))
      (if _found_3
        (bind _output_get_2 (set `local.foundIndex` _index_3))
        (`KismetArrayLibrary.Array_Set` (`self.slots`) _output_get_2 (make `/Game/Blueprints/S_ItemSlot` (`local.localClass`) 1))
        (`self.UpdateSlotAtIndex` (`local.foundIndex`))
        (if (> (`local.localAmount`) 1)
          (`self.addItem` (`local.localClass`) (- (`local.localAmount`) 1))
          (`self.UpdateCraftingMenu`)
          (return true)
          (else
            (`self.UpdateCraftingMenu`)
            (return true)))
        (else
          (return false))))))

(fn `amountAtIndex`
  (params (Index :type Integer))
  (returns (amount :type Integer))
  (return (`.Amount_8_68B4DFA949C468878DF3F7B69B4827B7` (break `/Game/Blueprints/S_ItemSlot` (`KismetArrayLibrary.Array_Get` (`self.slots`) Index)))))

(fn `findFreeStack`
  (params (itemClass :type "/Game/Blueprints/Item_Classes/BP_ItemMaster Class Reference"))
  (returns (found :type Boolean) (index :type Integer))
  (locals (localBool :type Boolean) (localIndex :type Integer))
  (for (_array_element _array_index) (`self.slots`)
    (bind (_itemclass _amount) (break `/Game/Blueprints/S_ItemSlot` _array_element))
    (if (`KismetSystemLibrary.IsValidClass` _itemclass)
      (if (and (== _itemclass itemClass) (< _amount (`self.maxStackSize`)))
        (set `local.localBool` true)
        (set `local.localIndex` _array_index)
        (break))))
  (return (`local.localBool`) (`local.localIndex`)))

(fn `getEmptySlot`
  (returns (index :type Integer) (found :type Boolean))
  (locals (localBool :type Boolean) (localIndex :type Integer))
  (for (_array_element _array_index) (`self.slots`)
    (if (not (`KismetSystemLibrary.IsValidClass` (`.ItemClass_5_307DBBD14BEB1EB4821A59ABFDAAF86F` (break `/Game/Blueprints/S_ItemSlot` _array_element))))
      (set `local.localBool` true)
      (set `local.localIndex` _array_index)
      (break)))
  (return (`local.localIndex`) (`local.localBool`)))

(fn `getItemInfo`
  (params (Index :type Integer))
  (returns (empty :type Boolean) (item :type "/Game/Blueprints/S_Item Structure") (amount :type Integer))
  (bind (_itemclass _amount) (break `/Game/Blueprints/S_ItemSlot` (`KismetArrayLibrary.Array_Get` (`self.slots`) Index)))
  (if (`KismetSystemLibrary.IsValidClass` _itemclass)
    (return false (defaults `/Game/Blueprints/BP_Inventory` _itemclass) _amount)
    (else
      (return true (struct) 0))))

(fn `GetTotalAmountOfItem`
  (params (Item :type "/Game/Blueprints/Item_Classes/BP_ItemMaster Class Reference"))
  (returns (TotalAmount :type Integer) (SlotIndices :type "Array of Integer"))
  (locals (localAmount :type Integer) (localSlotIndices :type "Array of Integer") (localItem :type "/Game/Blueprints/Item_Classes/BP_ItemMaster Class Reference"))
  (set `local.localItem` Item)
  (for (_array_element _array_index) (`self.slots`)
    (bind (_itemclass _amount) (break `/Game/Blueprints/S_ItemSlot` _array_element))
    (if (`KismetSystemLibrary.IsValidClass` _itemclass)
      (if (== _itemclass (`local.localItem`))
        (`KismetArrayLibrary.Array_Add` (`local.localSlotIndices`) _array_index)
        (set `local.localAmount` (+ (`local.localAmount`) _amount)))))
  (return (`local.localAmount`) (`local.localSlotIndices`)))

(fn `HideInventory`
  (`Widget.SetVisibility` (`self.Inventory Widget`) "Hidden")
  (set `self.isVisible` false)
  (`Widget.SetIsEnabled` (`self.Inventory Widget`) false)
  (return))

(fn `removeItem`
  (params (Item :type "/Game/Blueprints/Item_Classes/BP_ItemMaster Class Reference") (amount :type Integer))
  (returns (success :type Boolean))
  (locals (localSlotIndices :type "Array of Integer") (amountToRemove :type Integer))
  (bind (_totalamount _slotindices) (`self.GetTotalAmountOfItem` Item))
  (if (>= _totalamount amount)
    (set `local.localSlotIndices` _slotindices)
    (set `local.amountToRemove` amount)
    (for _array_element (`local.localSlotIndices`)
      (bind _amount (`self.amountAtIndex` _array_element))
      (if (< _amount (`local.amountToRemove`))
        (set `local.amountToRemove` (- (`local.amountToRemove`) _amount))
        (`self.removeItemAtIndex` _array_element _amount)
        (else
          (`self.removeItemAtIndex` _array_element (`local.amountToRemove`))
          (set `local.amountToRemove` 0)
          (break))))
    (return true)
    (else
      (return false))))

(fn `removeItemAtIndex`
  (params (index :type Integer) (amount :type Integer))
  (returns (success :type Boolean))
  (locals (localIndex :type Integer) (localAmount :type Integer))
  (bind _slots (`self.slots`))
  (bind _localindex (`local.localIndex`))
  (bind (_itemclass _amount) (break `/Game/Blueprints/S_ItemSlot` (`KismetArrayLibrary.Array_Get` _slots _localindex)))
  (set `local.localIndex` index)
  (set `local.localAmount` amount)
  (if (and (not (`self.slotEmpty` (`local.localIndex`))) (> (`local.localAmount`) 0))
    (if (>= (`local.localAmount`) (`self.amountAtIndex` (`local.localIndex`)))
      (`KismetArrayLibrary.Array_Set` (`self.slots`) (`local.localIndex`) (make `/Game/Blueprints/S_ItemSlot` null))
      (`self.UpdateSlotAtIndex` (`local.localIndex`))
      (`self.UpdateCraftingMenu`)
      (return true)
      (else
        (`KismetArrayLibrary.Array_Set` _slots _localindex (make `/Game/Blueprints/S_ItemSlot` _itemclass (- _amount (`local.localAmount`))))
        (`self.UpdateSlotAtIndex` (`local.localIndex`))
        (`self.UpdateCraftingMenu`)
        (return true)))
    (else
      (return false))))

(fn `ShowInventory`
  (`Widget.SetVisibility` (`self.Inventory Widget`) "Visible")
  (set `self.isVisible` true)
  (`Widget.SetIsEnabled` (`self.Inventory Widget`) true)
  (return))

(fn `slotEmpty`
  (params (index :type Integer))
  (returns (empty :type Boolean))
  (return (not (`KismetSystemLibrary.IsValidClass` (`.ItemClass_5_307DBBD14BEB1EB4821A59ABFDAAF86F` (break `/Game/Blueprints/S_ItemSlot` (`KismetArrayLibrary.Array_Get` (`self.slots`) index)))))))

(fn `UpdateCraftingMenu`
  (bind _craftingwidget (`/Game/GUI/W_Main.CraftingWidget` (`self.MainWidget`)))
  (bind _currentitemclass (`/Game/GUI/Crafting/W_CraftingMenu.CurrentItemClass` _craftingwidget))
  (if (`KismetSystemLibrary.IsValidClass` _currentitemclass)
    (`/Game/GUI/Crafting/W_CraftingMenu.UpdateDetailWindow` _craftingwidget _currentitemclass)
    (return)
    (else
      (return))))

(fn `UserConstructionScript`)