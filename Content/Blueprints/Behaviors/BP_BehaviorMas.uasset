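; BP_BehaviorMas is an actor Blueprint that serves as a lookup for per-customer item data.
; GetCustomerItemArray takes an index and switches between five item arrays for Boy, Girl, Merch, Strong and Wiz customer types.
; It also returns the matching GenValues entry as a float alongside the selected array.
; The event graph and construction script contain no logic.
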(fn `getCustomerItemArray`
  (params (num :type Integer))
  (returns (NewParam1 :type "Array of /Game/Blueprints/Item_Classes/BP_ItemMaster Class Reference") (NewParam :type "Float (double-precision)"))
  (bind _returnfloat (`self.returnFloat`))
  (set `self.returnFloat` (`KismetArrayLibrary.Array_Get` (`self.genValues`) num))
  (switch `int` num
    (:`0`
      (return (`self.itemsBoy`) _returnfloat))
    (:`1`
      (return (`self.itemsGirl`) _returnfloat))
    (:`2`
      (return (`self.itemsMerch`) _returnfloat))
    (:`3`
      (return (`self.itemsStrong`) _returnfloat))
    (:`4`
      (return (`self.itemsWiz`) _returnfloat))))

(fn `UserConstructionScript`)